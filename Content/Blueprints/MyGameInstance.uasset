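; Game instance that hosts and joins multiplayer sessions through Advanced Sessions nodes.
; CreateSession creates a session, then opens the VoiceChat level as a listen server.
; FindSession searches all server types, runs an empty loop over the results, then joins using the loop's final element.
; A failed search prints an error, while failed creation is unhandled.
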(event Custom|Create%20Session
  (|AdvancedSession 0 (Game|GetPlayerController 0) 100 0 false true false true true true false false false true
    (:OnSuccess
      (Game|OpenLevel(byName) "VoiceChat" true "listen"))))

(event Custom|Find%20Session
  (bind _results (|FindSessionsAdvanced (Game|GetPlayerController 0) 20 false "AllServers" 0 false false false true)
    (:OnSuccess
      (bind _output_get (Variables|Default|SetResults _results))
      (for _array_element _output_get
        _)
      (|JoinSession (Game|GetPlayerController 0) _array_element))
    (:OnFailure
      (Development|PrintString "Couldn't find online session!"))))